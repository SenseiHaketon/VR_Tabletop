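; Base pawn for a turn-based unit that can be picked up and dropped, with move, run and attack actions limited to one range each.
; Action events spawn range decals, while Tick range-checks the grabbed ghost or selected target in XY.
; Movement turns the pawn on the server via timeline, then runs AIMoveTo and flags the turn's action.
; Tick also replicates speed for animation and refreshes two health bars, tinted red for bosses.
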(event `/Game/Blueprints/Pickups/BP_PickupActorinterface.Pickup`
  (params (AttachTo :type "SceneComponent Object Reference") (Pawn :type "Pawn Object Reference") (PickupModeActive :type Boolean))
  ;[1 1 1] Pickup / Drop Events
  (`SceneComponent.K2_AttachToComponent` (`self.K2_GetRootComponent`) AttachTo "None" "KeepWorld" "KeepWorld" "KeepWorld" true)
  (`PrimitiveComponent.SetSimulatePhysics` (`self.SkeletalMesh`) false))

(event `MoveAction`
  (bind _returnvalue (`KismetMathLibrary.Conv_IntToDouble` (`self.speed`)))
  ;[1 1 1] Decal controls for Range Indicator
  (if (`|EnumEquality` (`self.action`) "NewEnumerator0")
    (bind _returnvalue_2 (`GameplayStatics.SpawnDecalAtLocation` "/Game/Materials/M_RangeDecal.M_RangeDecal" (`KismetMathLibrary.MakeVector` _returnvalue _returnvalue _returnvalue) (`self.K2_GetActorLocation`)))
    (set `self.MoveRangeDecal` _returnvalue_2)))

(event `ActivateMove`
  ;[1 1 1] Decal controls for Range Indicator
  (set `self.action` "NewEnumerator1"))

(event `/Game/Blueprints/Pickups/BP_PickupActorinterface.Drop`
  ;[1 1 1] Pickup / Drop Events
  (`self.K2_DetachFromActor` "KeepWorld" "KeepWorld" "KeepWorld")
  (`PrimitiveComponent.SetSimulatePhysics` (`self.SkeletalMesh`) true))

(event `RunAction`
  (bind _returnvalue (`KismetMathLibrary.Conv_IntToDouble` (* (`self.speed`) 2)))
  ;[1 1 1] Decal controls for Range Indicator
  (if (`|EnumEquality` (`self.action`) "NewEnumerator0")
    (bind _returnvalue_2 (`GameplayStatics.SpawnDecalAtLocation` "/Game/Materials/M_RangeDecal.M_RangeDecal" (`KismetMathLibrary.MakeVector` _returnvalue _returnvalue _returnvalue) (`self.K2_GetActorLocation`)))
    (set `self.MoveRangeDecal` _returnvalue_2)))

(event `ActivateRun`
  ;[1 1 1] Decal controls for Range Indicator
  (set `self.action` "NewEnumerator2"))

(event `AttackAction`
  (bind _returnvalue (`KismetMathLibrary.Conv_IntToDouble` (`self.range`)))
  ;[1 1 1] Decal controls for Range Indicator
  (if (`|EnumEquality` (`self.action`) "NewEnumerator0")
    (bind _returnvalue_2 (`GameplayStatics.SpawnDecalAtLocation` "/Game/Materials/M_RangeDecal.M_RangeDecal" (`KismetMathLibrary.MakeVector` _returnvalue _returnvalue _returnvalue) (`self.K2_GetActorLocation`)))
    (set `self.MoveRangeDecal` _returnvalue_2)
    (`self.ActivateAttack`)))

(event `ActivateAttack`
  ;[1 1 1] Decal controls for Range Indicator
  (set `self.action` "NewEnumerator3"))

(event `LookAtAndMove`
  (params (`Target Location` :type "Vector Structure"))
  (bind _scene (`self.Scene`))
  ;[1 1 1] Look at target
  (`/Engine/EditorBlueprintResources/ActorMacros.Switch Has Authority`
    (:`Authority`
      (bind (_direction _hure) (`Timeline|Timeline_0` :!via `PlayFromStart`)
        (:`Update`
          (bind _returnvalue (`self.K2_SetActorRotation` (`KismetMathLibrary.RLerp` (`SceneComponent.K2_GetComponentRotation` _scene) (`KismetMathLibrary.FindLookAtRotation` (`SceneComponent.K2_GetComponentLocation` _scene) `Target Location`) _hure)))
          (if _returnvalue
            (`self.MoveToLocation` `Target Location`)))))))

(event `MoveToLocation`
  (params (TargetLocation :type "Vector Structure"))
  ;[1 1 1] Move to target destination
  (switch `/Game/Structs/ActionEnum` (`self.action`)
    (:`NewEnumerator1`
      (set `FloatingPawnMovement.MaxSpeed` (`self.maxSpeed`) (`self.FloatingPawnMovement`)))
    (:`NewEnumerator2`
      (set `FloatingPawnMovement.MaxSpeed` (* (`self.maxSpeed`) 2.0) (`self.FloatingPawnMovement`))))
  (`|AIMoveTo` (`self.GetController` self) self TargetLocation
    (:`OnSuccess`
      (switch `/Game/Structs/ActionEnum` (`self.action`)
        (:`NewEnumerator1`
          (set `self.movedThisTurn` true))
        (:`NewEnumerator2`
          (set `self.ranThisTurn` true)))
      (set `self.action` "NewEnumerator0"))))

(event `ActivateNone`
  ;[1 1 1] Decal controls for Range Indicator
  (set `self.action` "NewEnumerator0")
  (`self.RemoveMoveRange`))

(event `RemoveMoveRange`
  (bind _moverangedecal (`self.MoveRangeDecal`))
  ;[1 1 1] Decal controls for Range Indicator
  (`/Engine/EditorBlueprintResources/StandardMacros.IsValid` _moverangedecal
    (:`Is Valid`
      (`ActorComponent.K2_DestroyComponent` _moverangedecal))))

(event `Attack`
  ;[1 1 1] Decal controls for Range Indicator
  (set `self.attackedThisTurn` true))

(event `self.ReceiveBeginPlay`
  (if (`self.isBoss`)
    (bind _asunit_healht_bar (cast `/Game/UI/UnitHealhtBar` (`WidgetComponent.GetUserWidgetObject` (`self.HealthBar`))))
    (`ProgressBar.SetFillColorAndOpacity` (`/Game/UI/UnitHealhtBar.HealthBar` _asunit_healht_bar) (struct :`R` 1.0 :`G` 0.030354 :`B` 0.070155 :`A` 1.0))
    (bind _asunit_healht_bar_2 (cast `/Game/UI/UnitHealhtBar` (`WidgetComponent.GetUserWidgetObject` (`self.HealhtBarBack`))))
    (`ProgressBar.SetFillColorAndOpacity` (`/Game/UI/UnitHealhtBar.HealthBar` _asunit_healht_bar_2) (struct :`R` 1.0 :`G` 0.028078 :`A` 1.0))))

(event `ResetTurn`
  ;[1 1 1] Reset turn
  (set `self.movedThisTurn` false)
  (set `self.attackedThisTurn` false)
  (set `self.ranThisTurn` false))

(event `self.ReceiveTick`
  (params (DeltaSeconds :type "Float (single-precision)"))
  (bind _action (`self.action`))
  (bind _speed (`self.speed`))
  (bind _returnvalue (`KismetMathLibrary.VSize` (`self.GetVelocity`)))
  (`|ExecutionSequence`
    (:`then_0`
      ;[1 1 1] Check if ghost is in Range
      (if (`self.isGrabbed`)
        (`/Engine/EditorBlueprintResources/StandardMacros.IsValid` (`self.ghostObject`)
          (:`Is Valid`
            (switch `/Game/Structs/ActionEnum` _action
              (:`NewEnumerator1`
                (`self.IsOtherActorInRange` (`self.ghostObject`) _speed))
              (:`NewEnumerator2`
                (`self.IsOtherActorInRange` (`self.ghostObject`) (* _speed 2))))))
        (else
          (`/Engine/EditorBlueprintResources/StandardMacros.IsValid` (`self.selectedTarget`)
            (:`Is Valid`
              (switch `/Game/Structs/ActionEnum` _action
                (:`NewEnumerator3`
                  (`self.IsOtherActorInRange` (`self.selectedTarget`) (`self.range`)))))))))
    (:`then_1`
      ;[1 1 1] Velocity Replication for Animations
      (`/Engine/EditorBlueprintResources/ActorMacros.Switch Has Authority`
        (:`Authority`
          (set `self.velocity` _returnvalue))
        (:`Remote`
          (if (`|EnumEquality` (`self.GetRemoteRole`) "ROLE_AutonomousProxy")
            (`self.ServerSetVelocity` _returnvalue)))))
    (:`then_2`
      (bind _asunit_healht_bar (cast `/Game/UI/UnitHealhtBar` (`WidgetComponent.GetUserWidgetObject` (`self.HealthBar`))))
      (`ProgressBar.SetPercent` (`/Game/UI/UnitHealhtBar.HealthBar` _asunit_healht_bar) (/ (`KismetMathLibrary.Conv_IntToDouble` (`self.health`)) (`KismetMathLibrary.Conv_IntToDouble` (`self.maxHealth`))))
      (`TextBlock.SetText` (`/Game/UI/UnitHealhtBar.HealthText` _asunit_healht_bar) (`KismetTextLibrary.Conv_StringToText` (`KismetStringLibrary.Concat_StrStr` (`KismetStringLibrary.Conv_IntToString` (`self.health`)) " / " (`KismetStringLibrary.Conv_IntToString` (`self.maxHealth`)))))
      (bind _asunit_healht_bar_2 (cast `/Game/UI/UnitHealhtBar` (`WidgetComponent.GetUserWidgetObject` (`self.HealhtBarBack`))))
      (`ProgressBar.SetPercent` (`/Game/UI/UnitHealhtBar.HealthBar` _asunit_healht_bar_2) (/ (`KismetMathLibrary.Conv_IntToDouble` (`self.health`)) (`KismetMathLibrary.Conv_IntToDouble` (`self.maxHealth`))))
      (`TextBlock.SetText` (`/Game/UI/UnitHealhtBar.HealthText` _asunit_healht_bar_2) (`KismetTextLibrary.Conv_StringToText` (`KismetStringLibrary.Concat_StrStr` (`KismetStringLibrary.Conv_IntToString` (`self.health`)) " / " (`KismetStringLibrary.Conv_IntToString` (`self.maxHealth`))))))))

(event `ServerSetVelocity`
  (params (value :type "Float (double-precision)"))
  ;[1 1 1] Velocity Replication for Animations
  (set `self.velocity` value))

(fn `IsOtherActorInRange`
  (params (OtherActor :type "Actor Object Reference") (Range :type Integer))
  (bind _returnvalue (`self.K2_GetActorLocation`))
  (if (<= (`KismetMathLibrary.VSize` (- (`KismetMathLibrary.MakeVector` (.x (`self.K2_GetActorLocation` OtherActor)) (.y (`self.K2_GetActorLocation` OtherActor)) (.z _returnvalue)) _returnvalue)) (`KismetMathLibrary.Conv_IntToDouble` Range))
    (set `self.isInRange?` true)
    (else
      (set `self.isInRange?` false))))

(fn `OnRep_TagRep`
  (set `self.Tags` (`self.TagRep`)))

(fn `UserConstructionScript`)