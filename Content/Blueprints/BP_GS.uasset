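; BP_GS, likely a Game State, runs a seconds countdown that marks the start of the game.
; OpenTick sets TickOpened and opens a gate on Tick, where a one-second Delay throttles the per-frame flow into a once-per-second decrement of Seconds.
; GameStarted turns true when Seconds drops below zero, and the same counter keeps decrementing afterward without a reset or end check.
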(event `self.ReceiveTick`
  (params (DeltaSeconds :type "Float (single-precision)"))
  (bind _seconds (`self.Seconds`))
  (`/Engine/EditorBlueprintResources/StandardMacros.Gate` true :!label _label
    (:`Exit`
      (`KismetSystemLibrary.Delay` 1.0)
      (if (`self.GameStarted`)
        (`/Engine/EditorBlueprintResources/StandardMacros.DecrementInt` (`self.Seconds`))
        (else
          (`/Engine/EditorBlueprintResources/StandardMacros.DecrementInt` _seconds
            (:`  `
              (if (< _seconds 0)
                (set `self.GameStarted` true)))))))))

(event `OpenTick`
  (set `self.tickOpened` true)
  (goto _label :!via `Open`))

(fn `UserConstructionScript`)