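; Main menu PlayerController that starts the menu in desktop or VR mode based on HMD name, and quits on Escape.
; InitHMD spawns a pawn through BP_GM_MainMenu, then adds MainMenuWB or, for Rift/SteamVR, enables the HMD.
; The VR path passes VRSettings to BP_GameInfoInstance to show the menu, setting IsVR false for SteamVR.
; ScalabilitySettings applies mirror, quality and resolution console commands; a vr.* variant is unwired.
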(event `Init HMD`
  (bind _returnvalue (`GameplayStatics.GetGameInstance`))
  (bind _vrsettings (`self.VRSettings`))
  ;[1 1 1] Initial Settings
  (switch `name` (`HeadMountedDisplayFunctionLibrary.GetHMDDeviceName`)
    (:`Default`
      (`self.Server_SpawnPawn` "/Script/Engine.DefaultPawn")
      (set `self.bShowMouseCursor` true)
      (bind _returnvalue_2 (`|CreateWidget` "/Game/UI/MainMenuWB.MainMenuWB_C" self))
      (`UserWidget.AddToViewport` _returnvalue_2 0))
    (:`OculusRift`
      (`self.Server_SpawnPawn` "/Game/Blueprints/Player/BP_PlayerPawn.BP_PlayerPawn_C" :!label _label)
      (setmembers `/Game/Structs/VRSettings` :`StructRef` (`self.VRSettings`) :`Controller_Mesh` "NewEnumerator0" :`Controller_Opacity` 15.0 :`Controller_Scale` 1.0 :`Controller_Skin_Vive` "NewEnumerator0" :`Enable_Screen_Messages` false :`Monitor_Output_Resolution` "1920x1080" :`GPU_VRAM` 4000 :`Show_Pointer_Controller` true :`Avatar_Color` (struct :`R` 0.8 :`G` 2.0 :`B` 5.0 :`A` 1.0) :`HMD_Mirror` "NewEnumerator4" :`HMD_Screen_Percentage` 130.0 :`TeleportRotationfromController` true)
      (`HeadMountedDisplayFunctionLibrary.EnableHMD` true)
      (`self.ScalabilitySettings`)
      (switch `name` (`HeadMountedDisplayFunctionLibrary.GetHMDDeviceName`)
        (:`OculusRift`
          (bind _asbp_game_info_instance (cast `/Game/Blueprints/BP_GameInfoInstance` _returnvalue))
          (set `/Game/Blueprints/BP_GameInfoInstance.VRSettings` _vrsettings _asbp_game_info_instance)
          (set `/Game/Blueprints/BP_GameInfoInstance.IsOculusRift` true _asbp_game_info_instance)
          (set `/Game/Blueprints/BP_GameInfoInstance.IsVR` true _asbp_game_info_instance)
          (`/Game/Blueprints/BP_GameInfoInstance.ShowMainMenu` _asbp_game_info_instance))
        (:`SteamVR`
          (bind _asbp_game_info_instance_2 (cast `/Game/Blueprints/BP_GameInfoInstance` _returnvalue))
          (set `/Game/Blueprints/BP_GameInfoInstance.VRSettings` _vrsettings _asbp_game_info_instance_2)
          (set `/Game/Blueprints/BP_GameInfoInstance.IsOculusRift` false _asbp_game_info_instance_2)
          (set `/Game/Blueprints/BP_GameInfoInstance.IsVR` false _asbp_game_info_instance_2)
          (`/Game/Blueprints/BP_GameInfoInstance.ShowMainMenu` _asbp_game_info_instance_2))))
    (:`SteamVR`
      (goto _label))))

(event `Key|Escape`
  (params (Key :type "Key Structure" :default "AnyKey"))
  ;[1 1 1] Initial Settings
  (:`Pressed`
    (`KismetSystemLibrary.QuitGame` null "Quit")))

(event `Server_SpawnPawn`
  (params (`Pawn Class` :type "Pawn Class Reference"))
  (`/Game/Blueprints/BP_GM_MainMenu.SpawnPawn` (cast `/Game/Blueprints/BP_GM_MainMenu` (`GameplayStatics.GetGameMode`) :!pure true) self `Pawn Class`))

(fn `ScalabilitySettings`
  (bind (_controller_mesh _controller_opacity _controller_scale _controller_skin_vive _enable_screen_messages _monitor_output_resolution _gpu_vram _show_pointer_controller _avatar_color _hmd_mirror _hmd_screen_percentage) (break `/Game/Structs/VRSettings` (`self.VRSettings`)))
  (`KismetSystemLibrary.ExecuteConsoleCommand` "stereo on" self)
  (switch `name` (`HeadMountedDisplayFunctionLibrary.GetHMDDeviceName`)
    (:`OculusRift`
      (`KismetSystemLibrary.ExecuteConsoleCommand` "hmd pdadaptive on" self)
      (`KismetSystemLibrary.ExecuteConsoleCommand` "hmd pdmin 2" self)
      (`KismetSystemLibrary.ExecuteConsoleCommand` (`KismetStringLibrary.Concat_StrStr` "stereo e=" (`KismetStringLibrary.Conv_DoubleToString` (`.IPD` (break `HmdUserProfile` (`OculusFunctionLibrary.GetUserProfile`))))) self)
      (switch `/Game/Structs/HMDMirrorMode` _hmd_mirror
        (:`NewEnumerator0`
          (`KismetSystemLibrary.ExecuteConsoleCommand` "hmd mirror mode 0" self))
        (:`NewEnumerator1`
          (`KismetSystemLibrary.ExecuteConsoleCommand` "hmd mirror mode 1" self))
        (:`NewEnumerator2`
          (`KismetSystemLibrary.ExecuteConsoleCommand` "hmd mirror mode 2" self))
        (:`NewEnumerator3`
          (`KismetSystemLibrary.ExecuteConsoleCommand` "hmd mirror mode 3" self))
        (:`NewEnumerator4`
          (`KismetSystemLibrary.ExecuteConsoleCommand` "hmd mirror mode 4" self))))
    (:`SteamVR`
      (switch `/Game/Structs/HMDMirrorMode` _hmd_mirror
        (:`NewEnumerator0`
          (`KismetSystemLibrary.ExecuteConsoleCommand` "hmd mirror 2" self))
        (:`NewEnumerator1`
          (`KismetSystemLibrary.ExecuteConsoleCommand` "hmd mirror 1" self :!label _label))
        (:`NewEnumerator2`
          (goto _label))
        (:`NewEnumerator3`
          (goto _label))
        (:`NewEnumerator4`
          (goto _label)))))
  (`KismetSystemLibrary.ExecuteConsoleCommand` (`KismetStringLibrary.Concat_StrStr` "r.ScreenPercentage " (`KismetStringLibrary.Conv_DoubleToString` _hmd_screen_percentage)))
  ;[0.3084 0 1] Scalability Settings
  ;;[1 1 1] View Distance Scale (0.1-2)
  (`KismetSystemLibrary.ExecuteConsoleCommand` "r.ViewDistanceScale 2" self)
  ;;[1 1 1] Post-process AA quality (0-3)
  (`KismetSystemLibrary.ExecuteConsoleCommand` "sg.AntiAliasingQuality 3" self)
  ;;[1 1 1] Shadow quality (0-3)
  (`KismetSystemLibrary.ExecuteConsoleCommand` "sg.ShadowQuality 3" self)
  ;;[1 1 1] Texture quality - MaxAnisotropy (2.5-0)
  (`KismetSystemLibrary.ExecuteConsoleCommand` "r.MaxAnisotropy 8" self)
  ;;[1 1 1] Texture quality - MipBias (2.5-0)
  (`KismetSystemLibrary.ExecuteConsoleCommand` "r.Streaming.MipBias 0" self)
  (`KismetSystemLibrary.ExecuteConsoleCommand` "r.SeparateTranslucency 0" self)
  (`KismetSystemLibrary.ExecuteConsoleCommand` "r.BloomQuality 0" self)
  ;;[1 1 1] Ensure it begins in fullscreen
  (`KismetSystemLibrary.ExecuteConsoleCommand` "fullscreen" self)
  ;[0.4845 0.2088 1] Initial Settings
  (if _enable_screen_messages
    (`KismetSystemLibrary.ExecuteConsoleCommand` "EnableAllScreenMessages" self)
    (else
      (`KismetSystemLibrary.ExecuteConsoleCommand` "DisableAllScreenMessages" self)))
  (`KismetSystemLibrary.ExecuteConsoleCommand` (`KismetStringLibrary.Concat_StrStr` "r.setres " _monitor_output_resolution) self)
  (`KismetSystemLibrary.ExecuteConsoleCommand` (`KismetStringLibrary.Concat_StrStr` "r.streaming.poolsize " (`KismetStringLibrary.Conv_IntToString` _gpu_vram)) self))

(fn `UserConstructionScript`)