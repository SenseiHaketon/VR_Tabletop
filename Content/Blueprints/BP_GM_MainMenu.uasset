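; Main menu game mode that sets up joining players and provides pawn spawning for them.
; On PostLogin it gathers the level's PlayerStarts into an array, then tells the BP_PC_MainMenu controller to initialize the HMD.
; A separate SpawnPawn event spawns a supplied pawn class at the first stored start and possesses it with the given controller.
; An older spawn-and-possess path for MainMenuPawn remains disconnected and never runs.
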(event `self.K2_PostLogin`
  (params (NewPlayer :type "PlayerController Object Reference"))
  (bind _outactors (`GameplayStatics.GetAllActorsOfClass` "/Script/Engine.PlayerStart"))
  (for _array_element _outactors
    (`KismetArrayLibrary.Array_AddUnique` (`self.Player1`) _array_element))
  (bind _asbp_pc_main_menu (cast `/Game/Blueprints/Player/BP_PC_MainMenu` NewPlayer))
  (`/Game/Blueprints/Player/BP_PC_MainMenu.Init HMD` _asbp_pc_main_menu))

(event `SpawnPawn`
  (params (PlayerController :type "PlayerController Object Reference") (PawnClass :type "Pawn Class Reference"))
  (bind _returnvalue (`|SpawnActorFromClass` PawnClass (`KismetMathLibrary.MakeTransform` (.location (`self.GetTransform` (`|GetArrayItem` (`self.Player1`)))) (.rotation (`self.GetTransform` (`|GetArrayItem` (`self.Player1`))))) "AlwaysSpawn" "OverrideRootScale" PlayerController))
  (`Controller.Possess` PlayerController _returnvalue))

(fn `UserConstructionScript`)