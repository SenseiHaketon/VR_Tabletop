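; BP_D12 is a twelve-sided physics die that can be picked up, dropped and read for its top face.
; Construction places twelve numbered marker components at icosahedron vertices; Tick takes the highest one's name as the rolled number.
; Pickup and Drop toggle physics and attachment; Destroyed increments total and per-face tallies in BP_TestGameState.
; A Fibonacci-sphere point generator and debug printing remain in unexecuted code.
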(event `self.ReceiveBeginPlay`
  (`SceneComponent.SetVisibility` (`self.Eyes`) false true))

(event `self.ReceiveTick`
  (params (DeltaSeconds :type "Float (single-precision)"))
  (for _array_element (`self.Sides`)
    (bind (_returnvalue_x _returnvalue_y _returnvalue_z) (`KismetMathLibrary.BreakVector` (`SceneComponent.K2_GetComponentLocation` _array_element)))
    (if (> _returnvalue_z (`self.TopHight`))
      (set `self.TopHight` _returnvalue_z)
      (set `self.TopNumber` (`KismetStringLibrary.Conv_StringToInt` (`KismetSystemLibrary.GetObjectName` _array_element)))))
  (set `self.TopHight` -1000.0))

(event `/Game/Blueprints/Pickups/BP_PickupActorinterface.Pickup`
  (params (AttachTo :type "SceneComponent Object Reference") (Pawn :type "Pawn Object Reference") (PickupModeActive :type Boolean))
  (`PrimitiveComponent.SetSimulatePhysics` (`self.PinkDice`) false)
  (`SceneComponent.K2_AttachToComponent` (`self.K2_GetRootComponent`) AttachTo "None" "KeepWorld" "KeepWorld" "KeepWorld" false))

(event `/Game/Blueprints/Pickups/BP_PickupActorinterface.Drop`
  (`PrimitiveComponent.SetSimulatePhysics` (`self.PinkDice`) true)
  (`self.K2_DetachFromActor` "KeepWorld" "KeepWorld" "KeepWorld"))

(event `self.ReceiveDestroyed`
  (bind _asbp_test_game_state (cast `/Game/Blueprints/Dice/BP_TestGameState` (`GameplayStatics.GetGameState`)))
  (bind _totaldiceresults (`/Game/Blueprints/Dice/BP_TestGameState.TotalDiceResults` _asbp_test_game_state))
  (`BlueprintMapLibrary.Map_Add` _totaldiceresults "NewEnumerator5" (+ (`BlueprintMapLibrary.Map_Find` _totaldiceresults "NewEnumerator5") 1))
  (bind _d12results (`/Game/Blueprints/Dice/BP_TestGameState.D12Results` _asbp_test_game_state))
  (`BlueprintMapLibrary.Map_Add` _d12results (`self.TopNumber`) (+ (`BlueprintMapLibrary.Map_Find` _d12results (`self.TopNumber`)) 1)))

(fn `MakeIcosahedron`
  (returns (Array :type "Array of Vector Structure"))
  (locals (A :type "Float (double-precision)" :default 0.525731) (B :type "Float (double-precision)" :default 0.850651))
  (return (`|MakeArray` (`KismetMathLibrary.MakeVector` (`self.Negate` (`local.A`)) 0.0 (`local.B`)) (`KismetMathLibrary.MakeVector` (`local.A`) 0.0 (`local.B`)) (`KismetMathLibrary.MakeVector` (`self.Negate` (`local.A`)) 0.0 (`self.Negate` (`local.B`))) (`KismetMathLibrary.MakeVector` (`local.A`) 0.0 (`self.Negate` (`local.B`))) (`KismetMathLibrary.MakeVector` 0.0 (`local.B`) (`local.A`)) (`KismetMathLibrary.MakeVector` 0.0 (`local.B`) (`self.Negate` (`local.A`))) (`KismetMathLibrary.MakeVector` 0.0 (`self.Negate` (`local.B`)) (`local.A`)) (`KismetMathLibrary.MakeVector` 0.0 (`self.Negate` (`local.B`)) (`self.Negate` (`local.A`))) (`KismetMathLibrary.MakeVector` (`local.B`) (`local.A`)) (`KismetMathLibrary.MakeVector` (`self.Negate` (`local.B`)) (`local.A`)) (`KismetMathLibrary.MakeVector` (`local.B`) (`self.Negate` (`local.A`))) (`KismetMathLibrary.MakeVector` (`self.Negate` (`local.B`)) (`self.Negate` (`local.A`))))))

(fn `Negate`
  (params (B :type "Float (double-precision)"))
  (returns (ReturnValue :type "Float (double-precision)"))
  (return (* -1 B)))

(fn `SphericalPenis`
  (params (Points :type Integer))
  (locals (inc :type "Float (double-precision)") (off :type "Float (double-precision)") (y :type "Float (double-precision)") (r :type "Float (double-precision)") (phi :type "Float (double-precision)") (k :type "Float (double-precision)") (n :type "Float (double-precision)"))
  (set `local.n` (`KismetMathLibrary.Conv_IntToDouble` Points))
  (for _index (range 1 (+ Points 1))
    (set `local.k` (`KismetMathLibrary.Conv_IntToDouble` _index))
    (set `local.inc` (* (`KismetMathLibrary.GetPI`) (- 3.0 (`KismetMathLibrary.Sqrt` 5.0))))
    (bind _output_get (set `local.off` (/ 2.0 (`local.n`))))
    (bind _output_get_2 (set `local.y` (- (* (`local.k`) _output_get) (+ 1.0 (/ _output_get 2.0)))))
    (set `local.r` (`KismetMathLibrary.Sqrt` (- 1.0 (`KismetMathLibrary.Square` _output_get_2))))
    (bind _output_get_3 (set `local.phi` (* (`local.k`) (`local.inc`))))
    (bind _returnvalue (`AddComponent|NODE_AddSceneComponent-0` :`bManualAttachment` true :`RelativeTransform` (`KismetMathLibrary.Conv_VectorToTransform` (`KismetMathLibrary.MakeVector` (* (`KismetMathLibrary.DegCos` _output_get_3) (`local.r`)) (`local.y`) (* (`KismetMathLibrary.DegSin` _output_get_3) (`local.r`))))))
    (`SceneComponent.K2_AttachToComponent` _returnvalue (`self.Eyes`) "None" "KeepWorld" "KeepWorld" "KeepWorld" true)
    (`KismetArrayLibrary.Array_Add` (`self.Sides`) _returnvalue)))

(fn `UserConstructionScript`
  (bind _output_get (set `self.Sides` (`|MakeArray` (`self.5`) (`self.4`) (`self.2`) (`self.12`) (`self.10`) (`self.8`) (`self.1`) (`self.3`) (`self.7`) (`self.9`) (`self.11`) (`self.6`))))
  (set `self.Pos` (`self.MakeIcosahedron`))
  (for (_array_element _array_index) _output_get
    (`SceneComponent.K2_SetRelativeLocation` _array_element (`|GetArrayItem` (`self.Pos`) _array_index) false false)))