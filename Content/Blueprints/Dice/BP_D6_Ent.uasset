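; Networked physics six-sided die that players can pick up and drop, tracking which face is up.
; Each tick it finds the highest of six side components and parses its name as TopNumber, then multicasts the mesh transform.
; Pickup disables physics and attaches the die to a given component; Drop detaches it and re-enables physics.
; Result display and game-state tallying are disconnected, and the table overlap check does nothing.
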(event `self.ReceiveBeginPlay`
  (`|ExecutionSequence`
    (:`then_0`
      (set `self.Sides` (`|MakeArray` (`self.1`) (`self.2`) (`self.3`) (`self.4`) (`self.5`) (`self.6`))))
    (:`then_1`
      (`self.Server_SetPhysics`))))

(event `Server_SetPhysics`
  (`PrimitiveComponent.SetSimulatePhysics` (`self.PinkDice`) true))

(event `UpdatePos`
  (`self.Multi_Physics` (`SceneComponent.K2_GetComponentToWorld` (`self.PinkDice`))))

(event `Multi_Physics`
  (params (Trans :type "Transform Structure"))
  (`SceneComponent.K2_SetWorldTransform` (`self.PinkDice`) Trans false false))

(event `self.ReceiveTick`
  (params (DeltaSeconds :type "Float (single-precision)"))
  (`|ExecutionSequence`
    (:`then_0`
      (for _array_element (`self.Sides`)
        (bind (_returnvalue_x _returnvalue_y _returnvalue_z) (`KismetMathLibrary.BreakVector` (`SceneComponent.K2_GetComponentLocation` _array_element)))
        (if (> _returnvalue_z (`self.TopHight`))
          (set `self.TopHight` _returnvalue_z)
          (set `self.TopNumber` (`KismetStringLibrary.Conv_StringToInt` (`KismetSystemLibrary.GetObjectName` _array_element)))))
      (set `self.TopHight` -1000.0))
    (:`then_2`
      (`self.UpdatePos`))))

(event `/Game/Blueprints/Pickups/BP_PickupActorinterface.Pickup`
  (params (AttachTo :type "SceneComponent Object Reference") (Pawn :type "Pawn Object Reference") (PickupModeActive :type Boolean))
  (`PrimitiveComponent.SetSimulatePhysics` (`self.PinkDice`) false)
  (`SceneComponent.K2_AttachToComponent` (`self.K2_GetRootComponent`) AttachTo "None" "KeepWorld" "KeepWorld" "KeepWorld" false))

(event `/Game/Blueprints/Pickups/BP_PickupActorinterface.Drop`
  (`PrimitiveComponent.SetSimulatePhysics` (`self.PinkDice`) true)
  (`self.K2_DetachFromActor` "KeepWorld" "KeepWorld" "KeepWorld"))

(event `self.ReceiveDestroyed`)

(event `self.Box.OnComponentBeginOverlap`
  (params (OverlappedComponent :type "PrimitiveComponent Object Reference") (OtherActor :type "Actor Object Reference") (OtherComp :type "PrimitiveComponent Object Reference") (OtherBodyIndex :type Integer) (bFromSweep :type Boolean) (SweepResult :type "HitResult Structure (by ref)"))
  (cast `/Game/Blueprints/Player/BP_PlayerPawn` (`GameplayStatics.GetPlayerPawn` 0))
  (if (`self.ActorHasTag` OtherActor "Table")
    _))

(fn `UserConstructionScript`)