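; Grabbable dice shaker that motion controllers pick up and drop by toggling physics and attachment.
; While attached, Tick presses it once the body rises 10 units above its Scene component, otherwise releasing it.
; On authority, pressing spawns requested cat D6s and D12s with random rotation and plays the cap-rotation timeline.
; Release reverses the cap and expires tracked dice; enter and exit triggers update that list, with exiting dice expiring later.
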(event `self.ReceiveBeginPlay`)

(event `Server_SetPhysics`
  (`PrimitiveComponent.SetSimulatePhysics` (`self.Shaker`) true))

(event `Multi_Physics`
  (params (Trans :type "Transform Structure"))
  (`SceneComponent.K2_SetWorldTransform` (`self.Shaker`) Trans false false))

(event `UpdatePos`
  (`self.Multi_Physics` (`SceneComponent.K2_GetComponentToWorld` (`self.Shaker`))))

(event `self.ReceiveTick`
  (params (DeltaSeconds :type "Float (single-precision)"))
  (bind (_returnvalue_x _returnvalue_y _returnvalue_z) (`KismetMathLibrary.BreakVector` (`SceneComponent.K2_GetComponentLocation` (`self.Shaker`))))
  (bind (_returnvalue_x_2 _returnvalue_y_2 _returnvalue_z_2) (`KismetMathLibrary.BreakVector` (`SceneComponent.K2_GetComponentLocation` (`self.Scene`))))
  (`/Engine/EditorBlueprintResources/StandardMacros.IsValid` (`self.GetAttachParentActor`)
    (:`Is Valid`
      (if (> (- _returnvalue_z _returnvalue_z_2) 10.0)
        (`/Engine/EditorBlueprintResources/StandardMacros.DoOnce` false :!label _label
          (:`Completed`
            (`self.press`)))
        (else
          (`self.release`))))
    (:`Is Not Valid`
      (`self.release`)
      (goto _label :!via `Reset`))))

(event `/Game/Blueprints/Pickups/BP_PickupActorinterface.Pickup`
  (params (AttachTo :type "SceneComponent Object Reference") (Pawn :type "Pawn Object Reference") (PickupModeActive :type Boolean))
  (`self.GetPickedUp` self (`self.Shaker`) AttachTo))

(event `press`
  (`self.Activate` "NewEnumerator0"))

(event `release`
  (`self.Activate` "NewEnumerator1"))

(event `/Game/Blueprints/Pickups/BP_PickupActorinterface.Drop`
  (`self.GetDropped` self (`self.Shaker`)))

(event `/Game/Blueprints/Dice/ActionObjectInterface.Activate`
  (params (InputEvent :type "/Game/Blueprints/Dice/EInputEvent Enum" :default "NewEnumerator0"))
  (bind _handle (`self.Handle`))
  (bind (_relativerotation_roll _relativerotation_pitch _relativerotation_yaw) (`KismetMathLibrary.BreakRotator` (`SceneComponent.RelativeRotation` _handle)))
  (switch `/Game/Blueprints/Dice/EInputEvent` InputEvent
    (:`NewEnumerator0`
      (`/Engine/EditorBlueprintResources/ActorMacros.Switch Has Authority`
        (:`Authority`
          (`self.SpawnDice`)
          (bind (_direction _rotation) (`Timeline|RotateCap` :!label _label_2)
            (:`Update`
              (`SceneComponent.K2_SetRelativeRotation` _handle (`KismetMathLibrary.MakeRotator` _rotation _relativerotation_pitch _relativerotation_yaw) false false))
            (:`Finished`
              (switch `ETimelineDirection` _direction))))))
    (:`NewEnumerator1`
      (`self.DestroyDice`)
      (goto _label_2 :!via `Reverse`))))

(event `SpawnDice`
  (bind _keys (`BlueprintMapLibrary.Map_Keys` (`self.RequestedDice`)))
  (for _array_element _keys
    (bind (_value _returnvalue) (`BlueprintMapLibrary.Map_Find` (`self.RequestedDice`) _array_element))
    (if _returnvalue
      (for _ (range 1 (+ _value 1))
        (switch `/Game/Blueprints/Dice/EDiceType` _array_element
          (:`NewEnumerator1`
            (set `self.DiceToSpawn` "/Game/Blueprints/Dice/BP_D6_Cat.BP_D6_Cat_C"))
          (:`NewEnumerator5`
            (set `self.DiceToSpawn` "/Game/Blueprints/Dice/BP_D12.BP_D12_C")))
        (bind _returnvalue_2 (`|SpawnActorFromClass` (`self.DiceToSpawn`) (`KismetMathLibrary.MakeTransform` (`SceneComponent.K2_GetComponentLocation` (`self.Spawnpoint`)) (`KismetMathLibrary.RandomRotator` false)) "AdjustIfPossibleButAlwaysSpawn" "OverrideRootScale" (`self.GetOwner`)))
        (`KismetArrayLibrary.Array_Add` (`self.Dice`) _returnvalue_2)))))

(event `DestroyDice`
  (for _array_element (`self.Dice`)
    (`/Engine/EditorBlueprintResources/StandardMacros.IsValid` _array_element
      (:`Is Valid`
        (`self.SetLifeSpan` _array_element 1.0))))
  (`KismetArrayLibrary.Array_Clear` (`self.Dice`)))

(event `self.EnterTrigger.OnComponentBeginOverlap`
  (params (OverlappedComponent :type "PrimitiveComponent Object Reference") (OtherActor :type "Actor Object Reference") (OtherComp :type "PrimitiveComponent Object Reference") (OtherBodyIndex :type Integer) (bFromSweep :type Boolean) (SweepResult :type "HitResult Structure (by ref)"))
  (cast `/Game/Blueprints/Dice/BP_D6_Cat` OtherActor
    (:`then`
      _)
    (:`CastFailed`
      (cast `/Game/Blueprints/Dice/BP_D12` OtherActor)))
  (`KismetArrayLibrary.Array_AddUnique` (`self.Dice`) OtherActor))

(event `self.ExitTrigger.OnComponentBeginOverlap`
  (params (OverlappedComponent :type "PrimitiveComponent Object Reference") (OtherActor :type "Actor Object Reference") (OtherComp :type "PrimitiveComponent Object Reference") (OtherBodyIndex :type Integer) (bFromSweep :type Boolean) (SweepResult :type "HitResult Structure (by ref)"))
  (cast `/Game/Blueprints/Dice/BP_D6_Cat` OtherActor
    (:`then`
      _)
    (:`CastFailed`
      (cast `/Game/Blueprints/Dice/BP_D12` OtherActor)))
  (`self.SetLifeSpan` OtherActor 5.0)
  (`KismetArrayLibrary.Array_RemoveItem` (`self.Dice`) OtherActor))

(fn `UserConstructionScript`)